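; Interactable world actor with a distance marker widget and an interact prompt widget.
; Each tick it measures meters to the player character, showing the marker with that whole-number distance at five or more and hiding it when closer.
; Prompt visibility follows a can-interact flag exposed through setter and getter functions.
; ChangeColor swaps the sphere's material; CanculateDistance and the construction script are empty.
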(event `self.ReceiveBeginPlay`
  (bind _asbp_task_01_character (cast `/Game/Task_01/Blueprints/BP_Task_01_Character` (`GameplayStatics.GetPlayerPawn` 0)))
  (set `self.As BP Task 01 Character` _asbp_task_01_character)
  (`SceneComponent.SetVisibility` (`self.W_Interact`) false false))

(event `self.ReceiveTick`
  (params (DeltaSeconds :type "Float (single-precision)"))
  (bind _returnvalue (`KismetMathLibrary.FTrunc` (/ (`KismetMathLibrary.Vector_Distance` (`self.K2_GetActorLocation` (`self.As BP Task 01 Character`)) (`self.K2_GetActorLocation`)) 100.0)))
  (bind _asw_marker (cast `/Game/Task_01/Widgets/W_Marker` (`WidgetComponent.GetUserWidgetObject` (`self.W_Marker`))))
  (if (>= _returnvalue 5)
    (`SceneComponent.SetVisibility` (`self.W_Marker`) true false)
    (`/Game/Task_01/Widgets/W_Marker.SetDistance` _asw_marker _returnvalue)
    (else
      (`SceneComponent.SetVisibility` (`self.W_Marker`) false false)))
  (`SceneComponent.SetVisibility` (`self.W_Interact`) (`self.bIsCanInteract`) false))

(fn `Canculate Distance`)

(fn `CanIteract`
  (returns (CanInteract :type Boolean))
  (return (`self.bIsCanInteract`)))

(fn `ChangeColor`
  (`PrimitiveComponent.SetMaterial` (`self.Sphere`) 0 "/Engine/MapTemplates/Materials/BasicAsset01.BasicAsset01"))

(fn `SetCanInteract`
  (params (bCanInteract :type Boolean))
  (set `self.bIsCanInteract` bCanInteract))

(fn `UserConstructionScript`)