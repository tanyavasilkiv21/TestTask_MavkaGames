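; Character Blueprint that detects which BP_Task_01_Actor the player is looking at and flags it as interactable.
; Each Tick, a short camera-forward trace finds the actor, then a second trace from the mesh to that hit point confirms line of sight before storing it and enabling interaction.
; The stored actor's flag clears only when the camera trace finds no task actor, not when the mesh trace fails.
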(event `self.ReceiveBeginPlay`)

(event `self.ReceiveTick`
  (params (DeltaSeconds :type "Float (single-precision)"))
  (bind _as_bp_task_01_actor (`self.As BP Task 01 Actor`))
  (bind _camera (`self.Camera`))
  (bind _returnvalue (`SceneComponent.K2_GetComponentLocation` _camera))
  (bind _outhit (`KismetSystemLibrary.LineTraceSingle` _returnvalue (+ _returnvalue (* (`KismetMathLibrary.GetForwardVector` (`SceneComponent.K2_GetComponentRotation` _camera)) 500.0)) "TraceTypeQuery1"))
  (bind _asbp_task_01_actor (cast `/Game/Task_01/Blueprints/BP_Task_01_Actor` (`.HitActor` (`GameplayStatics.BreakHitResult` _outhit)))
    (:`then`
      (bind _outhit_2 (`KismetSystemLibrary.LineTraceSingle` (`SceneComponent.K2_GetComponentLocation` (`self.Mesh`)) (`.Location` (`GameplayStatics.BreakHitResult` _outhit)) "TraceTypeQuery1"))
      (if (== (`.HitActor` (`GameplayStatics.BreakHitResult` _outhit_2)) _asbp_task_01_actor)
        (bind _output_get (set `self.As BP Task 01 Actor` _asbp_task_01_actor))
        (`/Game/Task_01/Blueprints/BP_Task_01_Actor.SetCanInteract` _output_get true)))
    (:`CastFailed`
      (if (`KismetSystemLibrary.IsValid` _as_bp_task_01_actor)
        (`/Game/Task_01/Blueprints/BP_Task_01_Actor.SetCanInteract` _as_bp_task_01_actor false)))))

(fn `UserConstructionScript`)