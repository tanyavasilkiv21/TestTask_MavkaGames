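; Task 04 character for exercising replication of objects and components, with a W_Print widget added to the viewport on BeginPlay.
; Tab calls an RPC that flip-flops Value1 on Obj, then multicasts the value and object name for printing.
; The server-gated construction of Obj is disconnected, so nothing here assigns it.
; CreateReplicatedComponent adds a BP_ReplicatedComponent on the server and prints its name, but is not called here.
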(event `self.ReceiveBeginPlay`
  (bind _returnvalue (`|CreateWidget` "/Game/Task_04/W_Print.W_Print_C"))
  (`UserWidget.AddToViewport` _returnvalue 0))

(event `RPC_FlipFlop`
  (bind _obj (`self.Obj`))
  (bind _isa (`/Engine/EditorBlueprintResources/StandardMacros.FlipFlop`)
    (:`A`
      _)
    (:`B`
      _))
  (bind _output_get (set `/Game/Task_04/BP_ObjectForReplication.Value1` _isa _obj))
  (`self.Multicast_PrintFlipFlop` _output_get (`KismetStringLibrary.Conv_StringToName` (`KismetSystemLibrary.GetObjectName` _obj))))

(event `Key|Tab`
  (params (Key :type "Key Structure"))
  (:`Pressed`
    (`self.RPC_FlipFlop`)))

(event `Multicast_PrintFlipFlop`
  (params (`Value 1` :type Boolean) (ObjName :type Name))
  (`KismetSystemLibrary.PrintString` (`KismetStringLibrary.Conv_BoolToString` `Value 1`))
  (`KismetSystemLibrary.PrintString` (`KismetStringLibrary.Conv_NameToString` ObjName)))

(fn `CreateReplicatedComponent`
  (returns (ReplicatedComponent :type "/Game/Task_04/BP_ReplicatedComponent Object Reference"))
  (if (`KismetSystemLibrary.IsServer`)
    (bind _returnvalue (`|AddComponentByClass` "/Game/Task_04/BP_ReplicatedComponent.BP_ReplicatedComponent_C"))
    (`KismetSystemLibrary.PrintString` (`KismetSystemLibrary.GetObjectName` _returnvalue))
    (return _returnvalue)))

(fn `UserConstructionScript`)