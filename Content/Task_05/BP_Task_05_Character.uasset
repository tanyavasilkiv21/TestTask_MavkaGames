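; BP_Task_05_Character is a Blueprint that moves itself along the spline of a BP_Trajectory actor once play begins.
; On BeginPlay it finds the trajectory and starts a timeline whose track maps to distance along the spline, setting location with a fixed upward offset, plus rotation.
; TimeToComplete, exposed through getter and setter functions, feeds straight into the timeline's play rate every update, so larger values move it faster despite the name.
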(event `self.ReceiveBeginPlay`
  (bind _returnvalue (`GameplayStatics.GetActorOfClass` "/Game/Task_05/BP_Trajectory.BP_Trajectory_C"))
  (set `self.Trajectory` _returnvalue)
  (`self.Move Obj`))

(event `Move Obj`
  (`TimelineComponent.SetPlayRate` (`self.Move Obj T`) (`self.time to complete`))
  (bind (_direction _movetrack) (`Timeline|Move Obj T` :!via `PlayFromStart`)
    (:`Update`
      (bind (_returnvalue_location _returnvalue_rotation) (`KismetMathLibrary.BreakTransform` (`SplineComponent.GetTransformAtDistanceAlongSpline` (`/Game/Task_05/BP_Trajectory.Spline` (`self.Trajectory`)) (`KismetMathLibrary.Lerp` 0.0 (`SplineComponent.GetSplineLength` (`/Game/Task_05/BP_Trajectory.Spline` (`self.Trajectory`))) _movetrack) "World" false)))
      (`self.K2_SetActorLocationAndRotation` (+ _returnvalue_location (0.0 0.0 138.0)) _returnvalue_rotation)
      (`TimelineComponent.SetPlayRate` (`self.Move Obj T`) (`self.time to complete`)))))

(fn `GetTimeToComplete`
  (returns (NewParam :type "Float (double-precision)"))
  (return (`self.time to complete`)))

(fn `SetTimeToComplete`
  (params (ParamTime :type "Float (double-precision)"))
  (set `self.time to complete` ParamTime))

(fn `UserConstructionScript`)